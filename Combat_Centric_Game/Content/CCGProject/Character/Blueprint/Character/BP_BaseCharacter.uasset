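; BP_BaseCharacter is a base character Blueprint that provides a shared ranged attack and placeholder weapon-point queries.
; RangeAttack spawns the given projectile class at GetMuzzle, rotated toward the target actor's location, and sets its Source to this character.
; GetMuzzle, GetWeaponTop and GetWeaponBottom are stubs returning zero vectors, apparently meant for child classes to override.
; The event graph and construction script contain no logic.
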(fn `GetMuzzle`
  (returns (Position :type "Vector Structure"))
  (return (0.0 0.0 0.0)))

(fn `GetWeaponBottom`
  (returns (Position :type "Vector Structure"))
  (return (0.0 0.0 0.0)))

(fn `GetWeaponTop`
  (returns (Position :type "Vector Structure"))
  (return (0.0 0.0 0.0)))

(fn `RangeAttack`
  (params (Projectile :type "/Game/CCGProject/Character/Monster/XBotMage/BP_XBM_Projectile Class Reference") (Target :type "/Game/CCGProject/Character/Blueprint/Character/BP_BaseCharacter Object Reference"))
  (bind _position (`self.GetMuzzle`))
  (bind _returnvalue (`|SpawnActorFromClass` Projectile (`KismetMathLibrary.MakeTransform` _position (`KismetMathLibrary.FindLookAtRotation` _position (`self.K2_GetActorLocation` Target))) "AlwaysSpawn" "MultiplyWithRoot" null null))
  (set `/Game/CCGProject/Character/Monster/XBotMage/BP_XBM_Projectile.Source` self _returnvalue))

(fn `UserConstructionScript`)