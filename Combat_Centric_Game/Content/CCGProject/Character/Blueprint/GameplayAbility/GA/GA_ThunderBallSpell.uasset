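; Gameplay ability for the player's thunder ball spell, which lobs a damaging projectile along the player's aimed velocity.
; On commit it clears the trajectory, flags the player as spell-attacking and plays the cast montage.
; A montage-timed gameplay event spawns BP_ThunderBall under gravity, handing it a damage effect spec with a SetByCaller rate.
; Montage completion, blend-out or interruption ends the ability and resets the player's spell flags.
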(event `self.K2_ActivateAbility`
  (bind _returnvalue_owneractor (break `GameplayAbilityActorInfo` (`self.GetActorInfo`)))
  (bind _as_bp_player_1 (`self.As BP Player 1`))
  (bind _returnvalue (`self.K2_CommitAbility`))
  (if _returnvalue
    (bind _asbp_player_1 (cast `/Game/CCGProject/Character/Player/Blueprint/BP_Player1` _returnvalue_owneractor))
    (bind _output_get (set `self.As BP Player 1` _asbp_player_1))
    (set `/Game/CCGProject/Character/Player/Blueprint/BP_Player1.IsSpellAttacking` true _output_get)
    (`BaseCharacter.ClearTrajectory` _output_get)
    (`|PlayMontage` (`Character.Mesh` (`self.As BP Player 1`)) "/Game/CCGProject/Character/Player/Animations/Spell/Spell_Shoot_Montage_01_03.Spell_Shoot_Montage_01_03"
      (:`then`
        (`AbilityTask_WaitGameplayEvent.WaitGameplayEvent` (struct :`TagName` "Ability.Skill.ThunderBallSpell") null
          (:`EventReceived`
            (bind _returnvalue_2 (`AbilitySystemBlueprintLibrary.AssignTagSetByCallerMagnitude` (`self.MakeOutgoingGameplayEffectSpec` (`self._damageEffect`)) (struct :`TagName` "Attack.DamageRate") (`self._damageRate`)))
            (bind _returnvalue_3 (`|SpawnActorFromClass` "/Game/CCGProject/Character/Player/Spell/BP_ThunderBall.BP_ThunderBall_C" (`SceneComponent.K2_GetComponentToWorld` (`Actor.RootComponent` (`self.As BP Player 1`))) "AlwaysSpawn" "MultiplyWithRoot" null null))
            (set `/Game/CCGProject/Character/Player/Spell/BP_ThunderBall.DamageEffectSpec` _returnvalue_2 _returnvalue_3)
            (bind _projectilemovement (`/Game/CCGProject/Character/Player/Spell/BP_ThunderBall.ProjectileMovement` _returnvalue_3))
            (set `MovementComponent.Velocity` (`BaseCharacter._projectileVelocity` (`self.As BP Player 1`)) _projectilemovement)
            (set `ProjectileMovementComponent.ProjectileGravityScale` 1.0 _projectilemovement))))
      (:`OnCompleted`
        (`self.K2_EndAbility` :!label _label)
        (set `/Game/CCGProject/Character/Player/Blueprint/BP_Player1.IsSpell ` false _as_bp_player_1)
        (set `/Game/CCGProject/Character/Player/Blueprint/BP_Player1.IsSpellAttacking` false _as_bp_player_1))
      (:`OnBlendOut`
        (goto _label))
      (:`OnInterrupted`
        (goto _label)))
    (else
      (`self.K2_EndAbility`))))