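; BP_Horse is a rideable horse the player can possess, with forward/back movement, look and adjustable spring-arm camera.
; Overlapping the RidePosition component binds HorseRide to BP_Player1's ride event, and leaving unbinds it.
; Riding stores the player, possesses the horse and shows a stand-in Player component.
; IA_Ride dismounts by moving the stored player to UnRidePosition, repossessing them and hiding the stand-in.
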(event `EnhancedInput|/Game/CCGProject/Controller/InputAction/IA_CameraLength`
  (params (ActionValue :type "Float (double-precision)") (ElapsedSeconds :type "Float (double-precision)") (TriggeredSeconds :type "Float (double-precision)") (InputAction :type "InputAction Object Reference" :default "/Game/CCGProject/Controller/InputAction/IA_CameraLength.IA_CameraLength"))
  (bind _springarm (`self.SpringArm`))
  ;[1 1 1] CameraLength
  (:`Triggered`
    (set `SpringArmComponent.TargetArmLength` (`KismetMathLibrary.FClamp` (+ (`SpringArmComponent.TargetArmLength` _springarm) (* ActionValue 50.0)) 300.0 600.0) _springarm)))

(event `EnhancedInput|/Game/CCGProject/Controller/InputAction/IA_Move`
  (params (ActionValue :type "Vector2D Structure") (ElapsedSeconds :type "Float (double-precision)") (TriggeredSeconds :type "Float (double-precision)") (InputAction :type "InputAction Object Reference" :default "/Game/CCGProject/Controller/InputAction/IA_Move.IA_Move"))
  ;[1 1 1] Move
  (:`Triggered`
    (bind _output_get (set `self.ForwardInput` ActionValue_Y))
    (`self.AddMovementInput` (`self.GetActorForwardVector`) _output_get))
  (:`Completed`
    (set `self.ForwardInput` 0.0)))

(event `EnhancedInput|/Game/CCGProject/Controller/InputAction/IA_CameraPosition`
  (params (ActionValue :type "Vector2D Structure") (ElapsedSeconds :type "Float (double-precision)") (TriggeredSeconds :type "Float (double-precision)") (InputAction :type "InputAction Object Reference" :default "/Game/CCGProject/Controller/InputAction/IA_CameraPosition.IA_CameraPosition"))
  ;[1 1 1] CameraPosition
  (:`Triggered`
    (`SceneComponent.K2_AddLocalOffset` (`self.SpringArm`) (`KismetMathLibrary.MakeVector` 0.0 ActionValue_X ActionValue_Y) false false)))

(event `EnhancedInput|/Game/CCGProject/Controller/InputAction/IA_Look`
  (params (ActionValue :type "Vector2D Structure") (ElapsedSeconds :type "Float (double-precision)") (TriggeredSeconds :type "Float (double-precision)") (InputAction :type "InputAction Object Reference" :default "/Game/CCGProject/Controller/InputAction/IA_Look.IA_Look"))
  ;[1 1 1] Look
  (:`Triggered`
    (`self.AddControllerYawInput` ActionValue_X)
    (`self.AddControllerPitchInput` ActionValue_Y)))

(event `self.RidePosition.OnComponentBeginOverlap`
  (params (OverlappedComponent :type "PrimitiveComponent Object Reference") (OtherActor :type "Actor Object Reference") (OtherComp :type "PrimitiveComponent Object Reference") (OtherBodyIndex :type Integer) (bFromSweep :type Boolean) (SweepResult :type "HitResult Structure (by ref)"))
  (bind _asbp_player_1 (cast `/Game/CCGProject/Character/Player/Blueprint/BP_Player1` OtherActor))
  (add `/Game/CCGProject/Character/Player/Blueprint/BP_Player1.HorseRide` _asbp_player_1 (delegate `HorseRide`)))

(event `self.RidePosition.OnComponentEndOverlap`
  (params (OverlappedComponent :type "PrimitiveComponent Object Reference") (OtherActor :type "Actor Object Reference") (OtherComp :type "PrimitiveComponent Object Reference") (OtherBodyIndex :type Integer))
  (bind _asbp_player_1 (cast `/Game/CCGProject/Character/Player/Blueprint/BP_Player1` OtherActor))
  (remove `/Game/CCGProject/Character/Player/Blueprint/BP_Player1.HorseRide` _asbp_player_1 (delegate `HorseRide`)))

(event `HorseRide`
  (bind _asbp_player_1 (cast `/Game/CCGProject/Character/Player/Blueprint/BP_Player1` (`GameplayStatics.GetPlayerCharacter` 0)))
  (set `self.As BP Player 1` _asbp_player_1)
  (`Controller.Possess` (`GameplayStatics.GetPlayerController` 0) self)
  (`SceneComponent.SetVisibility` (`self.Player`) true false))

(event `EnhancedInput|/Game/CCGProject/Controller/InputAction/IA_Ride`
  (params (ActionValue :type Boolean) (ElapsedSeconds :type "Float (double-precision)") (TriggeredSeconds :type "Float (double-precision)") (InputAction :type "InputAction Object Reference" :default "/Game/CCGProject/Controller/InputAction/IA_Ride.IA_Ride"))
  (bind _as_bp_player_1 (`self.As BP Player 1`))
  (:`Started`
    (`/Engine/EditorBlueprintResources/StandardMacros.IsValid` (`self.As BP Player 1`)
      (:`Is Valid`
        (`self.K2_SetActorTransform` _as_bp_player_1 (`SceneComponent.K2_GetComponentToWorld` (`self.UnRidePosition`)) false false)
        (`Controller.Possess` (`GameplayStatics.GetPlayerController` 0) _as_bp_player_1)
        (`SceneComponent.SetVisibility` (`self.Player`) false true)))))

(fn `UserConstructionScript`)