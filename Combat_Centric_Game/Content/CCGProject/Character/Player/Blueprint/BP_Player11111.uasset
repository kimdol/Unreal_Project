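; Player character Blueprint that handles walking, running and looking through Enhanced Input.
; BeginPlay adds the player controller mapping context, and the run action sets a flag that doubles the move axes.
; Move input is stored in side and forward variables, applied along the control rotation's right and forward vectors, and zeroed on release.
; Look input feeds controller yaw and pitch directly.
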(event `self.ReceiveBeginPlay`
  ;[1 1 1] InputMapping
  (bind `_as플레이어_컨트롤러` (cast `PlayerController` (`self.GetController`)))
  (`/Engine/EditorBlueprintResources/StandardMacros.IsValid` `_as플레이어_컨트롤러`
    (:`Is Valid`
      (`EnhancedInputSubsystemInterface.AddMappingContext` (pcsubsystem `EnhancedInputLocalPlayerSubsystem` `_as플레이어_컨트롤러`) "/Game/CCGProject/Controller/IMC_PlayerController.IMC_PlayerController" 0 (struct)))))

(event `EnhancedInput|/Game/CCGProject/Controller/InputAction/IA_Move`
  (params (ActionValue :type "Vector2D Structure") (ElapsedSeconds :type "Float (double-precision)") (TriggeredSeconds :type "Float (double-precision)") (InputAction :type "InputAction Object Reference" :default "/Game/CCGProject/Controller/InputAction/IA_Move.IA_Move"))
  (bind _returnvalue (`self.GetControlRotation`))
  ;[1 1 1] Move
  (:`Triggered`
    (if (`self.IsRun`)
      (set `self.SideInput` (* ActionValue_X 2.0))
      (set `self.ForwardInput` (* ActionValue_Y 2.0))
      (else
        (set `self.SideInput` ActionValue_X)
        (set `self.ForwardInput` ActionValue_Y)))
    (`self.AddMovementInput` (`KismetMathLibrary.GetRightVector` _returnvalue) (`self.SideInput`))
    (`self.AddMovementInput` (`KismetMathLibrary.GetForwardVector` _returnvalue) (`self.ForwardInput`)))
  (:`Completed`
    (set `self.SideInput` 0.0)
    (set `self.ForwardInput` 0.0)))

(event `EnhancedInput|/Game/CCGProject/Controller/InputAction/IA_Run`
  (params (ActionValue :type Boolean) (ElapsedSeconds :type "Float (double-precision)") (TriggeredSeconds :type "Float (double-precision)") (InputAction :type "InputAction Object Reference" :default "/Game/CCGProject/Controller/InputAction/IA_Run.IA_Run"))
  ;[1 1 1] Run
  (:`Triggered`
    (set `self.IsRun` ActionValue :!label _label))
  (:`Completed`
    (goto _label)))

(event `EnhancedInput|/Game/CCGProject/Controller/InputAction/IA_Look`
  (params (ActionValue :type "Vector2D Structure") (ElapsedSeconds :type "Float (double-precision)") (TriggeredSeconds :type "Float (double-precision)") (InputAction :type "InputAction Object Reference" :default "/Game/CCGProject/Controller/InputAction/IA_Look.IA_Look"))
  ;[1 1 1] Look
  (:`Triggered`
    (`self.AddControllerPitchInput` ActionValue_Y)
    (`self.AddControllerYawInput` ActionValue_X)))

(fn `UserConstructionScript`)