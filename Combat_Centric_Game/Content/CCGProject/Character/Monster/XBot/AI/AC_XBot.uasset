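; AC_XBot is the AI controller for the XBot monster, running its behavior tree on possession.
; Perception updates that sense an actor tagged Player cancel the reset timer and write IsInSight and TargetActor to the Blackboard.
; Any other update, including one from a non-player actor, starts a two-second timer that clears both keys, giving a grace period after sight loss.
; A debug "Hello" prints on every perception update.
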(event `self.ReceivePossess`
  (params (PossessedPawn :type "Pawn Object Reference"))
  (`self.RunBehaviorTree` "/Game/CCGProject/Character/Monster/XBot/AI/BT_MonsterXBot.BT_MonsterXBot"))

(event `ResetSight`
  (bind _blackboard (`self.Blackboard`))
  (`BlackboardComponent.SetValueAsBool` _blackboard (`self.IsInSight`) false)
  (`BlackboardComponent.SetValueAsObject` _blackboard (`self.TargetActor`) null))

(event `self.AIPerception.OnTargetPerceptionUpdated`
  (params (Actor :type "Actor Object Reference") (Stimulus :type "AIStimulus Structure"))
  (bind _blackboard (`self.Blackboard`))
  (`KismetSystemLibrary.PrintString` "Hello")
  (if (and (`self.ActorHasTag` Actor "Player") (`.bSuccessfullySensed` (break `AIStimulus` Stimulus)))
    (`KismetSystemLibrary.K2_ClearAndInvalidateTimerHandle` (`self.ResetTimer`))
    (`BlackboardComponent.SetValueAsBool` _blackboard (`self.IsInSight`) true)
    (`BlackboardComponent.SetValueAsObject` _blackboard (`self.TargetActor`) Actor)
    (else
      (bind _returnvalue (`KismetSystemLibrary.K2_SetTimerDelegate` (delegate `ResetSight`) 2.0))
      (set `self.ResetTimer` _returnvalue))))

(fn `UserConstructionScript`)