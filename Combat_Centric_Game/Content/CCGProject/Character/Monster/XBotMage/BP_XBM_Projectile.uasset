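; BP_XBM_Projectile is the XBotMage monster's projectile, which damages the player on overlap.
; When it overlaps a BP_Player1, it builds a DamageEffect gameplay effect spec from the Source's ability system component, with Attack.DamageRate set by caller.
; It applies that spec to the player's ability system component, then destroys itself; overlaps with other actors are ignored.
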(event `self.ReceiveActorBeginOverlap`
  (params (OtherActor :type "Actor Object Reference"))
  (bind _returnvalue (`AbilitySystemBlueprintLibrary.GetAbilitySystemComponent` (`self.Source`)))
  (bind _asbp_player_1 (cast `/Game/CCGProject/Character/Player/Blueprint/BP_Player1` OtherActor))
  (bind _returnvalue_2 (`AbilitySystemBlueprintLibrary.AssignTagSetByCallerMagnitude` (`AbilitySystemComponent.MakeOutgoingSpec` _returnvalue (`self.DamageEffect`) 1.0 (`AbilitySystemComponent.MakeEffectContext` _returnvalue)) (struct :`TagName` "Attack.DamageRate") 1.0))
  (`AbilitySystemComponent.BP_ApplyGameplayEffectSpecToTarget` (`AbilitySystemBlueprintLibrary.GetAbilitySystemComponent` (`self.Source`)) _returnvalue_2 (`AbilitySystemBlueprintLibrary.GetAbilitySystemComponent` _asbp_player_1))
  (`self.K2_DestroyActor`))

(fn `UserConstructionScript`)